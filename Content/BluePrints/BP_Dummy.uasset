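; BP_Dummy is a target that can be stealth-assassinated from behind, playing the victim half of a paired knife animation.
; An overlap radius shows the assassination prompt widget to BP_ThirdPersonCharacter, and Tick turns it toward the player camera.
; StealthBackAssasin plays the montage, hides the prompt and returns a reference location and the dummy's rotation to position the attacker.
; It also triggers Ragdoll, which uses delays to play the death sound, then enable mesh physics.
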(event OnComponentBeginOverlap(AssasinationRadius)
  (params (OverlappedComponent :type Primitive%20Component%20Object%20Reference) (OtherActor :type Actor%20Object%20Reference) (OtherComp :type Primitive%20Component%20Object%20Reference) (OtherBodyIndex :type Integer) (bFromSweep :type Boolean) (SweepResult :type Hit%20Result%20Structure%20%28by%20ref%29))
  ;[1 1 1] 可暗杀UI
  (Utilities|Casting|CastToBP_ThirdPersonCharacter OtherActor)
  (Rendering|SetVisibility (Variables|Default|GetAssasinate%20Widget) true false))

(event OnComponentEndOverlap(AssasinationRadius)
  (params (OverlappedComponent :type Primitive%20Component%20Object%20Reference) (OtherActor :type Actor%20Object%20Reference) (OtherComp :type Primitive%20Component%20Object%20Reference) (OtherBodyIndex :type Integer))
  ;[1 1 1] 可暗杀UI
  (Utilities|Casting|CastToBP_ThirdPersonCharacter OtherActor)
  (Rendering|SetVisibility (Variables|Default|GetAssasinate%20Widget) false false))

(event Custom|Ragdoll
  ;[1 1 1] 死亡后加物理碰撞效果
  (Utilities|FlowControl|Sequence
    (:then_0
      (Utilities|FlowControl|Delay 2.5)
      (Physics|SetSimulatePhysics (Variables|Character|GetMesh) true))
    (:then_1
      ;[1 1 1] 死亡音效
      (Utilities|FlowControl|Delay 1.5)
      (Audio|PlaySoundatLocation "/Game/Audio/Grunts-Hits/SC_Death.SC_Death" (Transformation|GetActorLocation) "0, 0, 0" 1.0 1.0 0.0 "/Game/Audio/SA_Character.SA_Character" 0 0 0))))

(event EventBeginPlay)

(event Collision|EventActorBeginOverlap
  (params (OtherActor :type Actor%20Object%20Reference)))

(event EventTick
  (params (DeltaSeconds :type Float%20%28single-precision%29))
  ;[1 1 1] 暗杀ui随玩家视角旋转
  (Transformation|SetWorldRotation (Variables|Default|GetAssasinate%20Widget) (Math|Rotator|FindLookatRotation (Transformation|GetWorldLocation (Variables|Default|GetAssasinate%20Widget)) (.location (Transformation|GetWorldTransform (Variables|/Script/Engine.PlayerCameraManager|GetTransformComponent (Game|GetPlayerCameraManager 0))))) false false))

(fn ConstructionScript)

(fn StealthBackAssasin
  ;[1 1 1] 被暗杀
  (Animation|PlayAnimMontage "/Game/Characters/RPG_Characters/Animantion/Assasination/Paired_Knife_Stealth_KidneyAndNeck_Vic_Montage.Paired_Knife_Stealth_KidneyAndNeck_Vic_Montage" 1.0 "None")
  (CallFunction|Ragdoll)
  (Rendering|SetVisibility (Variables|Default|GetAssasinate%20Widget) false false)
  (return (Transformation|GetWorldLocation (Variables|Default|GetAssasin%20REF)) (Transformation|GetActorRotation)))