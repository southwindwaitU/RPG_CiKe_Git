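; Player stats component that tracks health and stamina for BP_ThirdPersonCharacter and keeps its HUD widget in sync.
; It caches the owning character one tick after BeginPlay, and each stat change directly sets the HUD bars and texts.
; Decrease functions return whether the stat is depleted, updating the HUD before clamping to zero.
; Restore functions cap at the maximum, while max increases leave current values unchanged.
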(event EventBeginPlay
  ;[1 1 1] 获得player变量
  (Utilities|FlowControl|DelayUntilNextTick)
  (bind _asbp_third_person_character (Utilities|Casting|CastToBP_ThirdPersonCharacter (Components|GetOwner)))
  (Variables|Default|SetBP%20Player%20Character _asbp_third_person_character))

(event EventTick
  (params (DeltaSeconds :type Float%20%28single-precision%29)))

(fn DecreaseHealth
  (params (Damage :type Float%20%28double-precision%29))
  (bind _bp_player_character (Variables|Default|GetBP%20Player%20Character))
  (bind _hud_widget (Variables|/Game/ThirdPerson/Blueprints/BP_ThirdPersonCharacter.BP_ThirdPersonCharacter_C|GetHUD%20Widget _bp_player_character))
  ;[1 1 1] 收到伤害扣血并检查是否死亡
  (if (> (Variables|Health|GetCurrent%20Health) 0.0)
    (bind _output_get (Variables|Health|SetCurrent%20Health (- (Variables|Health|GetCurrent%20Health) Damage)))
    (Progress|SetPercent (Variables|/Game/UI/WB_HUD.WB_HUD_C|GetHealthBar _hud_widget) (/ _output_get (Variables|Health|GetMax%20Health)))
    (Rendering|Components|TextRender|SetText (Variables|/Game/UI/WB_HUD.WB_HUD_C|GetHealthText _hud_widget) (Utilities|Text|ToText(Float) (Variables|Health|GetCurrent%20Health) "HalfToEven"))
    (if (<= (Variables|Health|GetCurrent%20Health) 0.0)
      (Variables|Health|SetCurrent%20Health 0.0)
      (else
        (return false))))
  (return true))

(fn IncreaseMaxHealth
  (params (HealthIncremention :type Float%20%28double-precision%29))
  (bind _bp_player_character (Variables|Default|GetBP%20Player%20Character))
  (bind _hud_widget (Variables|/Game/ThirdPerson/Blueprints/BP_ThirdPersonCharacter.BP_ThirdPersonCharacter_C|GetHUD%20Widget _bp_player_character))
  ;[1 1 1] 增加最大血量
  (Variables|Health|SetMax%20Health (+ HealthIncremention (Variables|Health|GetMax%20Health)))
  (Rendering|Components|TextRender|SetText (Variables|/Game/UI/WB_HUD.WB_HUD_C|GetHealthText _hud_widget) (Utilities|Text|ToText(Float) (Variables|Health|GetCurrent%20Health) "HalfToEven"))
  (Progress|SetPercent (Variables|/Game/UI/WB_HUD.WB_HUD_C|GetHealthBar _hud_widget) (/ (Variables|Health|GetCurrent%20Health) (Variables|Health|GetMax%20Health)))
  (Rendering|Components|TextRender|SetText (Variables|/Game/UI/WB_HUD.WB_HUD_C|GetMaxHealthText _hud_widget) (Utilities|Text|ToText(Float) (Variables|Health|GetMax%20Health) "HalfToEven")))

(fn DecreaseStamina
  (params (Stamina%20Depleted :type Float%20%28double-precision%29))
  (bind _bp_player_character (Variables|Default|GetBP%20Player%20Character))
  (bind _hud_widget (Variables|/Game/ThirdPerson/Blueprints/BP_ThirdPersonCharacter.BP_ThirdPersonCharacter_C|GetHUD%20Widget _bp_player_character))
  ;[1 1 1] 消耗耐力并判断是否耗尽耐力
  (if (> (Variables|Stamina|GetCurrent%20Stamina) 0.0)
    (Variables|Stamina|SetCurrent%20Stamina (- (Variables|Stamina|GetCurrent%20Stamina) Stamina%20Depleted))
    (Progress|SetPercent (Variables|/Game/UI/WB_HUD.WB_HUD_C|GetStaminaBar _hud_widget) (/ (Variables|Stamina|GetCurrent%20Stamina) (Variables|Stamina|GetMax%20Stamina)))
    (Rendering|Components|TextRender|SetText (Variables|/Game/UI/WB_HUD.WB_HUD_C|GetStaminaText _hud_widget) (Utilities|Text|ToText(Float) (Variables|Stamina|GetCurrent%20Stamina) "HalfToEven"))
    (if (<= (Variables|Stamina|GetCurrent%20Stamina) 0.0)
      (Variables|Stamina|SetCurrent%20Stamina 0.0)
      (else
        (return false))))
  (return true))

(fn IncreaseMaxStamina
  (params (Stamina%20Incremention :type Float%20%28double-precision%29))
  (bind _bp_player_character (Variables|Default|GetBP%20Player%20Character))
  (bind _hud_widget (Variables|/Game/ThirdPerson/Blueprints/BP_ThirdPersonCharacter.BP_ThirdPersonCharacter_C|GetHUD%20Widget _bp_player_character))
  ;[1 1 1] 增加最大耐力
  (Variables|Stamina|SetMax%20Stamina (+ Stamina%20Incremention (Variables|Stamina|GetMax%20Stamina)))
  (Progress|SetPercent (Variables|/Game/UI/WB_HUD.WB_HUD_C|GetStaminaBar _hud_widget) (/ (Variables|Stamina|GetCurrent%20Stamina) (Variables|Stamina|GetMax%20Stamina)))
  (Rendering|Components|TextRender|SetText (Variables|/Game/UI/WB_HUD.WB_HUD_C|GetStaminaText _hud_widget) (Utilities|Text|ToText(Float) (Variables|Stamina|GetCurrent%20Stamina) "HalfToEven"))
  (Rendering|Components|TextRender|SetText (Variables|/Game/UI/WB_HUD.WB_HUD_C|GetMaxStaminaText _hud_widget) (Utilities|Text|ToText(Float) (Variables|Stamina|GetMax%20Stamina) "HalfToEven")))

(fn IncreaseCurrentHealth
  (params (Added%20Health :type Float%20%28double-precision%29))
  (bind _bp_player_character (Variables|Default|GetBP%20Player%20Character))
  (bind _hud_widget (Variables|/Game/ThirdPerson/Blueprints/BP_ThirdPersonCharacter.BP_ThirdPersonCharacter_C|GetHUD%20Widget _bp_player_character))
  ;[1 1 1] 回复血量
  (Variables|Health|SetCurrent%20Health (+ Added%20Health (Variables|Health|GetCurrent%20Health)))
  (if (> (Variables|Health|GetCurrent%20Health) (Variables|Health|GetMax%20Health))
    (Variables|Health|SetCurrent%20Health (Variables|Health|GetMax%20Health)))
  (Progress|SetPercent (Variables|/Game/UI/WB_HUD.WB_HUD_C|GetHealthBar _hud_widget) (/ (Variables|Health|GetCurrent%20Health) (Variables|Health|GetMax%20Health)))
  (Rendering|Components|TextRender|SetText (Variables|/Game/UI/WB_HUD.WB_HUD_C|GetHealthText _hud_widget) (Utilities|Text|ToText(Float) (Variables|Health|GetCurrent%20Health) "HalfToEven")))

(fn IncreaseCurrentStamina
  (params (Added%20Stamina :type Float%20%28double-precision%29))
  (bind _bp_player_character (Variables|Default|GetBP%20Player%20Character))
  (bind _hud_widget (Variables|/Game/ThirdPerson/Blueprints/BP_ThirdPersonCharacter.BP_ThirdPersonCharacter_C|GetHUD%20Widget _bp_player_character))
  ;[1 1 1] 回复耐力
  (Variables|Stamina|SetCurrent%20Stamina (+ Added%20Stamina (Variables|Stamina|GetCurrent%20Stamina)))
  (if (> (Variables|Stamina|GetCurrent%20Stamina) (Variables|Stamina|GetMax%20Stamina))
    (Variables|Stamina|SetCurrent%20Stamina (Variables|Stamina|GetMax%20Stamina)))
  (Progress|SetPercent (Variables|/Game/UI/WB_HUD.WB_HUD_C|GetStaminaBar _hud_widget) (/ (Variables|Stamina|GetCurrent%20Stamina) (Variables|Stamina|GetMax%20Stamina)))
  (Rendering|Components|TextRender|SetText (Variables|/Game/UI/WB_HUD.WB_HUD_C|GetStaminaText _hud_widget) (Utilities|Text|ToText(Float) (Variables|Stamina|GetCurrent%20Stamina) "HalfToEven")))